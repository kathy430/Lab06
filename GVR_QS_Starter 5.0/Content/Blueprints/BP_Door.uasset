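; BP_Door is an interactable sliding door that moves its Door component between DoorStart and DoorEnd.
; The Interact event plays TimelineDoorDriver when DoorClosed is true and reverses it otherwise.
; The timeline's Driver track lerps the door's relative location without sweep.
; DoorClosed flips on every timeline update rather than on completion, so its value after a move depends on the update count.
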(event EventBeginPlay)

(event Collision|EventActorBeginOverlap
  (params (OtherActor :type Actor%20Object%20Reference)))

(event EventTick
  (params (DeltaSeconds :type Float%20%28single-precision%29)))

(event EventInteract
  (if (Variables|Default|GetDoorClosed)
    (bind _driver (Timeline|Timeline%20-%20Door%20Driver Play)
      (:Update
        (Transformation|SetRelativeLocation (Variables|Default|GetDoor) (Math|Vector|Lerp(Vector) (Variables|DoorSetup|GetDoorStart) (Variables|DoorSetup|GetDoorEnd) _driver) false false)
        (if (Variables|Default|GetDoorClosed)
          (Variables|Default|SetDoorClosed false)
          (else
            (Variables|Default|SetDoorClosed true)))))
    (else
      (Timeline|Timeline%20-%20Door%20Driver Reverse))))

(fn ConstructionScript)