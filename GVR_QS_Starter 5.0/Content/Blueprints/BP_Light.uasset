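; BP_Light is a light actor that switches on and off through an Interact event.
; Interact toggles the visibility of the Sphere and PointLight components without propagating to their children.
; It then checks whether the point light is visible and sets the TextRender to the LightOn or LightOff text to match.
; All logic lives in that event, with no active BeginPlay, Tick, overlap or construction logic.
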(event EventBeginPlay)

(event Collision|EventActorBeginOverlap
  (params (OtherActor :type Actor%20Object%20Reference)))

(event EventTick
  (params (DeltaSeconds :type Float%20%28single-precision%29)))

(event EventInteract
  (bind _pointlight (Variables|Default|GetPointLight))
  ;[1 1 1] Comment
  (Rendering|ToggleVisibility (Variables|Default|GetSphere) false)
  (Rendering|ToggleVisibility _pointlight false)
  (if (Rendering|IsVisible _pointlight)
    (Rendering|Components|TextRender|SetText (Variables|Default|GetTextRender) (Variables|Default|GetLightOn))
    (else
      (Rendering|Components|TextRender|SetText (Variables|Default|GetTextRender) (Variables|Default|GetLightOff)))))

(fn ConstructionScript)