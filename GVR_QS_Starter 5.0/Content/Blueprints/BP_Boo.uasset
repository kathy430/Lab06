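; BP_Boo is a Boo-style ghost that creeps toward the player only while it is not being rendered.
; Each tick, a recent-render check plays a timeline when seen or reverses it when unseen, driving the Translucency parameter on the sphere's dynamic material.
; While unseen, it also moves straight toward the player pawn at Speed, without sweeping for collision.
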(event EventBeginPlay
  (bind _returnvalue (Rendering|Material|CreateDynamicMaterialInstance (Variables|Default|GetSphere) 0 0 "None" :!class /Script/Engine.PrimitiveComponent))
  (Variables|Default|SetTranslucent%20Material%20Instance _returnvalue)
  (Transformation|SetActorRotation "0,150.000000, 0"))

(event EventTick
  (params (DeltaSeconds :type Float%20%28single-precision%29))
  (bind _returnvalue (Transformation|GetActorLocation))
  (if (Class|Actor|WasRecentlyRendered 0.2)
    (bind _alpha (Timeline|Timeline_Alpha Play)
      (:Update
        (Rendering|Material|SetScalarParameterValue (Variables|Default|GetTranslucent%20Material%20Instance) "Translucency" _alpha :!class /Script/Engine.MaterialInstanceDynamic)))
    (else
      (Utilities|FlowControl|Sequence
        (:then_0
          (Timeline|Timeline_Alpha Reverse))
        (:then_1
          (Transformation|SetActorLocation (+ (* (Math|Vector|Normalize (- (Transformation|GetActorLocation (Game|Player|GetPlayerPawn 0)) _returnvalue)) DeltaSeconds (Variables|Default|Getspeed)) _returnvalue) false false))))))

(fn ConstructionScript)