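; BP_Character is a player character that looks around with the mouse and uses gaze to interact with actors or teleport.
; Each tick, a visibility line trace from the camera, debug-drawn, stores any hit actor implementing BP_Interact as the interaction target.
; Click sends InteractMessage to that target, or otherwise teleports to the traced impact point with a vertical offset, provided the trace hit something blocking.
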(event Custom|GazeCheck
  (bind _camera (Variables|Default|GetCamera))
  (bind _returnvalue (Transformation|GetWorldLocation _camera))
  ;[1 1 1] Gaze check
  (bind _outhit (Collision|LineTraceByChannel _returnvalue (+ _returnvalue (* (Math|Vector|GetForwardVector _camera) 2000)) "TraceTypeQuery1" false 0 "ForOneFrame"))
  (if (Utilities|DoesObjectImplementInterface (.HitActor (Collision|BreakHitResult _outhit)) "/Game/Blueprints/BP_Interact.BP_Interact_C")
    (Variables|Default|SetinteractingActor (.HitActor (Collision|BreakHitResult _outhit)))
    (else
      (Variables|Default|SetinteractingActor 0))))

(event EventTick
  (params (DeltaSeconds :type Float%20%28single-precision%29))
  (CallFunction|GazeCheck))

(event Input|ActionEvents|InputActionClick
  (params (Key :type Key%20Structure :default "None"))
  (bind _interactingactor (Variables|Default|GetinteractingActor))
  (:Pressed
    (Utilities|IsValid _interactingactor
      (:Is%20Valid
        (Class|BPInteract|Interact(Message) _interactingactor))
      (:Is%20Not%20Valid
        (CallFunction|Teleport (.ImpactPoint (Collision|BreakHitResult (stale Custom|GazeCheck _outhit))) (.bBlockingHit (Collision|BreakHitResult (stale Custom|GazeCheck _outhit))))))))

(event Input|AxisEvents|InputAxismouseX
  (params (AxisValue :type Float%20%28single-precision%29))
  ;[1 1 1] Input
  (Pawn|Input|AddControllerYawInput AxisValue))

(event Input|AxisEvents|InputAxismouseY
  (params (AxisValue :type Float%20%28single-precision%29))
  ;[1 1 1] Input
  (Pawn|Input|AddControllerPitchInput AxisValue))

(fn ConstructionScript)

(fn Teleport
  (params (Location :type Vector) (Blocking%20Hit :type Boolean))
  (if Blocking%20Hit
    (Transformation|SetActorLocation (+ Location "0,0.000000,88.000000") false false)))